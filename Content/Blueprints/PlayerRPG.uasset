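; PlayerRPG is the player character Blueprint, handling movement, look, jumping and incoming damage.
; Axis inputs drive movement along the actor's forward and right vectors and feed controller pitch and yaw for looking.
; Space Bar triggers Jump through a direct key binding.
; Any damage received is passed straight to HealthStat's ChangeHealth, with no sign change or other processing in this graph.
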(event Game|Damage|EventAnyDamage
  (params (Damage :type Float%20%28single-precision%29) (DamageType :type Damage%20Type%20Object%20Reference) (InstigatedBy :type Controller%20Object%20Reference) (DamageCauser :type Actor%20Object%20Reference))
  (Default|ChangeHealth (Variables|Default|GetHealthStat) Damage))

(event Input|AxisEvents|InputAxisMoveLR
  (params (AxisValue :type Float%20%28single-precision%29))
  ;[1 1 1] Input
  (Pawn|Input|AddMovementInput (Transformation|GetActorRightVector) AxisValue false))

(event Input|AxisEvents|InputAxisMoveUD
  (params (AxisValue :type Float%20%28single-precision%29))
  ;[1 1 1] Input
  (Pawn|Input|AddMovementInput (Transformation|GetActorForwardVector) AxisValue false))

(event Input|AxisEvents|InputAxisLookUD
  (params (AxisValue :type Float%20%28single-precision%29))
  ;[1 1 1] Input
  (Pawn|Input|AddControllerPitchInput AxisValue))

(event Input|AxisEvents|InputAxisLookRL
  (params (AxisValue :type Float%20%28single-precision%29))
  ;[1 1 1] Input
  (Pawn|Input|AddControllerYawInput AxisValue))

(event Input|KeyboardEvents|SpaceBar
  (params (Key :type Key%20Structure :default "AnyKey"))
  ;[1 1 1] Input
  (:Pressed
    (Character|Jump)))

(fn ConstructionScript)